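; RTS HUD that shows and hides a drag-selection rectangle on screen.
; On BeginPlay it creates a hidden WBP_SelectionFrame widget for the owning player and adds it to the viewport.
; DrawSelectionFrame reveals the widget, positions it with DPI scale removed and sizes it by dividing width and height by viewport scale.
; HideSelectionFrame hides it again.
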(event `self.ReceiveBeginPlay`
  (bind _returnvalue (`|CreateWidget` "/Game/TestTask/UI/WBP_SelectionFrame.WBP_SelectionFrame_C" (`self.GetOwningPlayerController`)))
  (bind _output_get (set `self.SelectionFrame` _returnvalue))
  (`UserWidget.AddToViewport` _output_get 0)
  (`Widget.SetVisibility` _output_get "Hidden"))

(event `self.ReceiveDrawSelectionFrame`
  (params (ScreenX :type "Float (single-precision)") (ScreenY :type "Float (single-precision)") (Width :type "Float (single-precision)") (Height :type "Float (single-precision)"))
  (bind _returnvalue (`WidgetLayoutLibrary.GetViewportScale`))
  (`Widget.SetVisibility` (`self.SelectionFrame`) "Visible")
  (`UserWidget.SetPositionInViewport` (`self.SelectionFrame`) (`KismetMathLibrary.MakeVector2D` ScreenX ScreenY) true)
  (`UserWidget.SetDesiredSizeInViewport` (`self.SelectionFrame`) (`KismetMathLibrary.MakeVector2D` (/ Width _returnvalue) (/ Height _returnvalue))))

(event `self.ReceiveHideSelectionFrame`
  (`Widget.SetVisibility` (`self.SelectionFrame`) "Hidden"))

(fn `UserConstructionScript`)